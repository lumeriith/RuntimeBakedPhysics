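; Jenga tower actor that builds a stack of floors on demand and can toggle its physics.
; CreateTower destroys previously spawned floors, then spawns JengaFloorBP actors upward from its location at EachHeight spacing, all sharing its rotation, and returns them.
; Freeze and Unfreeze switch physics simulation off and on for every static mesh component in those floors.
; The event graph and construction script are empty, so these functions need external callers.
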(event EventBeginPlay)

(event Collision|EventActorBeginOverlap
  (params (OtherActor :type Actor%20Object%20Reference)))

(event EventTick
  (params (DeltaSeconds :type Float%20%28single-precision%29)))

(fn ConstructionScript)

(fn CreateTower
  (params (Height :type Integer))
  (bind _spawned_floors (Variables|Default|GetSpawned%20Floors))
  (for _array_element (Variables|Default|GetSpawned%20Floors)
    (Actor|DestroyActor _array_element))
  (Utilities|Array|Clear (Variables|Default|GetSpawned%20Floors))
  (for _index (range 0 Height)
    (bind _returnvalue (Game|SpawnActorfromClass "/Game/JengaFloorBP.JengaFloorBP_C" (Math|Transform|MakeTransform (+ (Math|Vector|MakeVector 0.0 0.0 (* _index (Variables|Default|GetEach%20Height))) (Transformation|GetActorLocation)) (Transformation|GetActorRotation)) "Undefined" 0 0))
    (Utilities|Array|Add _spawned_floors _returnvalue))
  (return _spawned_floors))

(fn Freeze
  (for _array_element (Variables|Default|GetSpawned%20Floors)
    (for _array_element_2 (Actor|GetComponentsByClass _array_element "/Script/Engine.StaticMeshComponent")
      (bind _asstatic_mesh_component (Utilities|Casting|CastToStaticMeshComponent _array_element_2))
      (Physics|SetSimulatePhysics _asstatic_mesh_component false))))

(fn Unfreeze
  (for _array_element (Variables|Default|GetSpawned%20Floors)
    (for _array_element_2 (Actor|GetComponentsByClass _array_element "/Script/Engine.StaticMeshComponent")
      (bind _asstatic_mesh_component (Utilities|Casting|CastToStaticMeshComponent _array_element_2))
      (Physics|SetSimulatePhysics _asstatic_mesh_component true))))
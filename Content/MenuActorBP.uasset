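; Menu actor that shows the menu widget on BeginPlay and exposes functions for controlling a physics simulation of Zenga towers.
; Changing tower height clears the PhysScene, registers meshes of static objects, rebuilds each tower at the given height, adds its blocks as dynamic objects, then freezes it.
; Record, Play and Cancel forward to the PhysScene, with recording taking an interval and frame count.
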(event EventBeginPlay
  (bind _returnvalue (UserInterface|CreateWidget "/Game/MenuWidgetBP.MenuWidgetBP_C" 0 self))
  (UserInterface|Viewport|AddtoViewport _returnvalue 0))

(event Collision|EventActorBeginOverlap
  (params (OtherActor :type Actor%20Object%20Reference)))

(event EventTick
  (params (DeltaSeconds :type Float%20%28single-precision%29)))

(fn ConstructionScript)

(fn ChangeAllTowerHeight
  (params (height :type Integer))
  (Class|AdvPhysScene|ClearPhysObjects (Variables|Default|GetPhysScene))
  (for _array_element (Variables|Default|GetStaticObjects)
    (for _array_element_2 (Actor|GetComponentsByClass _array_element "/Script/Engine.StaticMeshComponent")
      (Class|AdvPhysScene|AddStaticObject (Variables|Default|GetPhysScene) _array_element_2)))
  (for _array_element_3 (Variables|Default|GetZengaTower)
    (bind _createdfloors (Default|CreateTower _array_element_3 height))
    (for _array_element_4 _createdfloors
      (for _array_element_5 (Actor|GetComponentsByClass _array_element_4 "/Script/Engine.StaticMeshComponent")
        (bind _asstatic_mesh_component (Utilities|Casting|CastToStaticMeshComponent _array_element_5))
        (Class|AdvPhysScene|AddDynamicObject (Variables|Default|GetPhysScene) _asstatic_mesh_component)))
    (Default|Freeze _array_element_3)))

(fn Record
  (params (Interval :type Float%20%28double-precision%29) (FrameCount :type Integer))
  (Class|AdvPhysScene|Record (Variables|Default|GetPhysScene) Interval FrameCount))

(fn Play
  (Class|AdvPhysScene|Play (Variables|Default|GetPhysScene)))

(fn Cancel
  (Class|AdvPhysScene|Cancel (Variables|Default|GetPhysScene)))
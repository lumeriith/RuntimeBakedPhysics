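; Actor Blueprint that builds a Zenga tower at runtime by stacking ZengaFloorBP actors, starting on BeginPlay with a hard-coded floor count.
; CreateTower first destroys and clears any previously tracked floors, so the tower can be rebuilt.
; It then spawns floors at the actor's location and rotation, offsetting each along world Z by EachHeight and tracking them in SpawnedFloors.
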(event EventBeginPlay
  (CallFunction|CreateTower 5))

(event Collision|EventActorBeginOverlap
  (params (OtherActor :type Actor%20Object%20Reference)))

(event EventTick
  (params (DeltaSeconds :type Float%20%28single-precision%29)))

(fn ConstructionScript)

(fn CreateTower
  (params (floors :type Integer))
  (bind _spawnedfloors (Variables|Default|GetspawnedFloors))
  (bind _result (Utilities|Set|ToArray _spawnedfloors))
  (for _array_element _result
    (Actor|DestroyActor _array_element))
  (Utilities|Set|Clear _spawnedfloors)
  (for _index (range 0 floors)
    (bind _returnvalue (Game|SpawnActorfromClass "/Game/ZengaFloorBP.ZengaFloorBP_C" (Math|Transform|MakeTransform (+ (Math|Vector|MakeVector 0.0 0.0 (* _index (Variables|Default|GeteachHeight))) (Transformation|GetActorLocation)) (Transformation|GetActorRotation)) "Undefined" 0 0))
    (Utilities|Set|Add (Variables|Default|GetspawnedFloors) _returnvalue)))